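; TelePawn is a pawn that finds and previews a teleport spot where its camera is looking.
; Each tick it line-traces along the camera's forward vector, accepts near-horizontal, upward-facing surfaces and marks the hit with a debug cylinder.
; The teleport call is not connected to any event, and TeleportToLocation ignores its Location input, setting the actor to the camera's relative XY at zero height.
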(event `self.ReceiveTick`
  (params (DeltaSeconds :type "Float (single-precision)"))
  (bind _camera (`self.Camera`))
  (`self.TraceGetTeleportLocation` (`SceneComponent.K2_GetComponentLocation` _camera) (`SceneComponent.GetForwardVector` _camera)))

(fn `TeleportToLocation`
  (params (Location :type "Vector Structure"))
  (bind (_relativelocation_x _relativelocation_y) (`KismetMathLibrary.BreakVector` (`SceneComponent.RelativeLocation` (`self.Camera`))))
  (`self.K2_SetActorLocation` (+ (0.0 0.0 0.0) (`KismetMathLibrary.MakeVector` _relativelocation_x _relativelocation_y))))

(fn `TraceGetTeleportLocation`
  (params (Position :type "Vector Structure") (ForwardVector :type "Vector Structure"))
  (bind _outhit (`KismetSystemLibrary.LineTraceSingle` Position (+ Position (* ForwardVector 10000.0)) "TraceTypeQuery2"))
  (bind (_bblockinghit _binitialoverlap _time _distance _location _impactpoint _normal) (`GameplayStatics.BreakHitResult` _outhit))
  (bind _output_get (set `self.CanTeleport` (> (`KismetMathLibrary.Dot_VectorVector` _normal (0.0 0.0 1.0)) 0.9)))
  (if _output_get
    (bind _output_get_2 (set `self.TeleportLocation` _location))
    (`KismetSystemLibrary.DrawDebugCylinder` _output_get_2 (+ _output_get_2 (* _normal 20.0)) 50.0 20 (struct :`R` 0.004949 :`G` 0.019227 :`B` 1.0 :`A` 1.0) 0.0 2.0)))

(fn `UserConstructionScript`)